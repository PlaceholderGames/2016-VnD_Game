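; Trigger box that lets a digger ant dig away a linked target actor.
; Until activated, it polls overlapping AI_Ant actors every Tick, and one with Dig set starts a looping Scale timer.
; Each timer step lowers the target's Z scale from Size, destroying both target and trigger when Size nearly equals a hardcoded flattened value, which assumes a fixed X/Y scale.
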(event EventBeginPlay)

(event Collision|EventActorBeginOverlap
  (params (OtherActor :type Actor%20Object%20Reference)))

(event EventTick
  (params (DeltaSeconds :type Float%20%28single-precision%29))
  ;[1 1 1] Detects when ants enter trigger box, if digger it will trigger the digging effect to destroy the box.
  (if (not (Variables|Default|GetisActive))
    (bind _array_element (Utilities|Array|ForEachLoopwithBreak (Collision|GetOverlappingActors "/Game/ThirdPersonBP/Blueprints/AI_Ant.AI_Ant_C" :!class /Script/Engine.Actor))
      (:LoopBody
        (bind _asai_ant (Utilities|Casting|CastToAI_Ant _array_element))
        (if (Variables|/Game/ThirdPersonBP/Blueprints/AI_Ant.AI_Ant_C|Getdig _asai_ant)
          (bind _returnvalue (Utilities|Time|SetTimerbyFunctionName 0 "Scale" 0.01 true))
          (Variables|Default|SetisActive true))))))

(event EventDestroyed
  ;[1 1 1] Detects when ants enter trigger box, if digger it will trigger the digging effect to destroy the box.
  (Utilities|Time|ClearandInvalidateTimerbyHandle (stale EventTick _returnvalue)))

(fn ConstructionScript)

(fn Scale
  (bind _targetactor (Variables|Default|GetTargetActor))
  (bind _output_get (Variables|Default|SetSize (- (Variables|Default|GetSize) "0, 0,0.010000")))
  (Transformation|SetActorScale3D _targetactor _output_get)
  (if (Math|Vector|Equal(Vector) (Variables|Default|GetSize) "2.000000,2.000000,0.010000" 0.0001)
    (Actor|DestroyActor _targetactor)
    (Actor|DestroyActor)))