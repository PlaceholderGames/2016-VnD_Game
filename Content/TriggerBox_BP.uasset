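; Trigger box that flattens a target actor and then removes it once anything overlaps its collision component.
; The overlap starts a fast looping timer calling Scale, which steps down the Z of a stored Size and applies it to TargetActor.
; When Size nearly equals a hard-coded flattened scale, both target and trigger are destroyed, and the Destroyed event clears the timer.
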(event OnComponentBeginOverlap(CollisionComponent)
  (params (OverlappedComponent :type Primitive%20Component%20Object%20Reference) (OtherActor :type Actor%20Object%20Reference) (OtherComp :type Primitive%20Component%20Object%20Reference) (OtherBodyIndex :type Integer) (bFromSweep :type Boolean) (SweepResult :type Hit%20Result%20Structure%20%28by%20ref%29))
  (bind _returnvalue (Utilities|Time|SetTimerbyFunctionName 0 "Scale" 0.01 true)))

(event EventBeginPlay)

(event Collision|EventActorBeginOverlap
  (params (OtherActor :type Actor%20Object%20Reference)))

(event EventDestroyed
  (Utilities|Time|ClearandInvalidateTimerbyHandle (stale OnComponentBeginOverlap(CollisionComponent) _returnvalue)))

(fn ConstructionScript)

(fn Scale
  (bind _targetactor (Variables|Default|GetTargetActor))
  (bind _output_get (Variables|Default|SetSize (- (Variables|Default|GetSize) "0, 0,0.010000")))
  (Transformation|SetActorScale3D _targetactor _output_get)
  (if (Math|Vector|Equal(Vector) (Variables|Default|GetSize) "2.000000,2.000000,0.010000" 0.0001)
    (Actor|DestroyActor _targetactor)
    (Actor|DestroyActor)))