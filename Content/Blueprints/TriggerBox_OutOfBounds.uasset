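; Out-of-bounds trigger box that destroys any actor entering it and can end the game once enough deaths are counted.
; Only overlapping actors that cast to AntSpawner, checked after the destroy call, increment AntsDead, which is compared against that actor's MaxAnts.
; At that limit it shows the end game menu, pauses the game, disables player input and reveals the mouse cursor.
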(event EventBeginPlay)

(event Collision|EventActorBeginOverlap
  (params (OtherActor :type Actor%20Object%20Reference))
  (bind _returnvalue (Game|GetPlayerController 0))
  (Actor|DestroyActor OtherActor)
  (bind _asant_spawner (Utilities|Casting|CastToAntSpawner OtherActor))
  (bind _output_get (Variables|Default|SetAntsDead (+ (Variables|Default|GetAntsDead) 1)))
  (if (>= _output_get (Variables|/Game/ThirdPersonBP/Blueprints/AntSpawner.AntSpawner_C|GetMax%20Ants _asant_spawner))
    (bind _returnvalue_2 (UserInterface|CreateWidget "/Game/Screens/Widgets/EndGameMenu_widget.EndGameMenu_widget_C"))
    (UserInterface|Viewport|AddtoViewport _returnvalue_2 0)
    (Game|SetGamePaused true)
    (Input|DisableInput (Game|GetPlayerCharacter 0) _returnvalue)
    (Variables|/Script/Engine.PlayerController|SetbShowMouseCursor _returnvalue true)))

(event EventTick
  (params (DeltaSeconds :type Float%20%28single-precision%29)))

(fn ConstructionScript)